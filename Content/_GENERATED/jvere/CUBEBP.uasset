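; CUBEBP is a shooting enemy that reacts to the top-down player character and can trigger the move to BUDDHALEVEL.
; PawnSensing turns it toward a seen BP_TopDownCharacter, then spawns a Bullet at its Arrow after a short delay.
; Damage reduces Health; at zero it destroys itself and decrements its own Enemies variable.
; Tick polls that variable and opens BUDDHALEVEL after a delay when it equals zero.
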(event OnSeePawn(PawnSensing)
  (params (Pawn :type Pawn%20Object%20Reference))
  (bind _asbp_top_down_character (Utilities|Casting|CastToBP_TopDownCharacter Pawn)
    (:then
      (Utilities|FlowControl|Sequence
        (:then_0
          (Transformation|SetActorRotation (Math|Rotator|FindLookatRotation (Transformation|GetActorLocation) (Transformation|GetActorLocation _asbp_top_down_character))))
        (:then_1
          (Utilities|FlowControl|Delay 1.0)
          (Game|SpawnActorfromClass "/Game/LevelPrototyping/Bullet/Bullet.Bullet_C" (Transformation|GetWorldTransform (Variables|Default|GetArrow)) "Undefined" "MultiplyWithRoot" 0 0))))
    (:CastFailed
      (Development|PrintText "Cast failed"))))

(event EventBeginPlay)

(event Collision|EventActorBeginOverlap
  (params (OtherActor :type Actor%20Object%20Reference)))

(event EventTick
  (params (DeltaSeconds :type Float%20%28single-precision%29))
  (Math|Float|CompareFloat (Variables|Default|GetEnemies) 0.0
    (:==
      (Utilities|FlowControl|Delay 5.0)
      (Game|OpenLevel(byObjectReference) "/Game/Westward/Levels/BUDDHALEVEL.BUDDHALEVEL"))))

(event Game|Damage|EventAnyDamage
  (params (Damage :type Float%20%28single-precision%29) (DamageType :type Damage%20Type%20Object%20Reference) (InstigatedBy :type Controller%20Object%20Reference) (DamageCauser :type Actor%20Object%20Reference))
  (bind _output_get (Variables|Default|SetHealth (- (Variables|Default|GetHealth) Damage)))
  (if (<= _output_get 0.0)
    (Actor|DestroyActor)
    (bind _result (Math|Float|DecrementFloat (Variables|Default|GetEnemies))
      (:%20%20
        (Variables|Default|SetEnemies _result)))))

(fn ConstructionScript)